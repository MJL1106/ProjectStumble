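; Base game mode for Stumble that handles respawning the player and resetting spawned level content.
; RespawnPlayer runs the reset, spawns a new actor of the given player's class at RespawnTransform, and has player controller 0 possess it.
; ResetActors destroys every actor tagged "Reset", then zeroes each Actor_Spawner's spawn count and restarts it through ResetSpawning.
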(event Custom|ResetActors
  (bind _outactors (Actor|GetAllActorswithTag "Reset"))
  (for _array_element _outactors
    (Actor|DestroyActor _array_element))
  (bind _outactors_2 (Actor|GetAllActorsOfClass "/Game/Stumble/Enemy/EnemySpawner/Actor_Spawner.Actor_Spawner_C"))
  (for _array_element_2 _outactors_2
    (Variables|/Game/Stumble/Enemy/EnemySpawner/Actor_Spawner.Actor_Spawner_C|SetTotal%20Spawned _array_element_2 0)
    (Default|ResetSpawning _array_element_2)))

(event Custom|Respawn%20Player
  (params (Player :type Character%20Object%20Reference))
  (CallFunction|ResetActors)
  (bind _returnvalue (Game|SpawnActorfromClass (Utilities|GetClass Player) (Variables|Default|GetRespawn%20Transform) "Undefined" "MultiplyWithRoot" 0 0))
  (Pawn|Possess (Game|GetPlayerController 0) _returnvalue))

(fn ConstructionScript)