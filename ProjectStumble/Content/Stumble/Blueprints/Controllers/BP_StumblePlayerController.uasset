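; BP_StumblePlayerController is the player controller that routes input to the controlled BP_StumbleCharacter.
; While the character is on a ladder, the MoveForward axis switches movement to Flying and moves it along the player character's up vector.
; Reload and Fire actions call the character's weapon functions, with Fire passing pressed or released state.
; A hardcoded L key triggers the character's door interaction.
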(event Input|ActionEvents|InputActionFire
  (params (Key :type Key%20Structure :default "None"))
  (bind _returnvalue (Pawn|GetControlledPawn))
  ;[1 1 1] Shooting
  (:Pressed
    (bind _asbp_stumble_character (Utilities|Casting|CastToBP_StumbleCharacter _returnvalue))
    (Default|Fire _asbp_stumble_character true))
  (:Released
    (bind _asbp_stumble_character_2 (Utilities|Casting|CastToBP_StumbleCharacter _returnvalue))
    (Default|Fire _asbp_stumble_character_2 false)))

(event Input|ActionEvents|InputActionReload
  (params (Key :type Key%20Structure :default "None"))
  ;[1 1 1] Reload
  (:Pressed
    (bind _asbp_stumble_character (Utilities|Casting|CastToBP_StumbleCharacter (Pawn|GetControlledPawn)))
    (Default|Reloading _asbp_stumble_character)))

(event Input|AxisEvents|InputAxisMoveForward
  (params (AxisValue :type Float%20%28single-precision%29))
  ;[1 1 1] Ladder Movement
  (bind _asbp_stumble_character (Utilities|Casting|CastToBP_StumbleCharacter (Pawn|GetControlledPawn)))
  (bind _isonladder (Default|GetIsonLadder _asbp_stumble_character))
  (if _isonladder
    (Pawn|Components|CharacterMovement|SetMovementMode (Variables|/Script/Engine.Character|GetCharacterMovement _asbp_stumble_character) "MOVE_Flying" 0)
    (Class|PawnMovementComponent|AddInputVector (Pawn|GetMovementComponent _asbp_stumble_character) (* (Transformation|GetActorUpVector (Game|GetPlayerCharacter 0)) AxisValue) false)))

(event Input|KeyboardEvents|L
  (params (Key :type Key%20Structure :default "None"))
  (:Pressed
    (bind _asbp_stumble_character (Utilities|Casting|CastToBP_StumbleCharacter (Pawn|GetControlledPawn)))
    (Default|DoorInteraction _asbp_stumble_character)))

(fn ConstructionScript)