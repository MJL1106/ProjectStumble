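; Enemy spawner actor for Stumble that spawns a configurable enemy class at its own transform, in single or wave mode.
; Single mode spawns one enemy at BeginPlay.
; Otherwise, the first Stumble character entering the Box starts MultiSpawn, which spawns batches and re-calls itself after a delay until MaxSpawn is reached.
; ResetSpawning clears Activated and repeats any single spawn, but leaves TotalSpawned untouched.
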(event OnComponentBeginOverlap(Box)
  (params (OverlappedComponent :type Primitive%20Component%20Object%20Reference) (OtherActor :type Actor%20Object%20Reference) (OtherComp :type Primitive%20Component%20Object%20Reference) (OtherBodyIndex :type Integer) (bFromSweep :type Boolean) (SweepResult :type Hit%20Result%20Structure%20%28by%20ref%29))
  (if (not (Variables|Default|GetSingle%20Spawn))
    (Utilities|Casting|CastToBP_StumbleCharacter OtherActor)
    (if (not (Variables|Default|GetActivated?))
      (CallFunction|MultiSpawn (Variables|Default|GetEnemy) (Transformation|GetActorTransform) (Variables|Default|GetNumber%20Of%20Enemies))
      (Variables|Default|SetActivated? true))))

(event Custom|MultiSpawn
  (params (Enemy :type Actor%20Class%20Reference) (SpawnTransform :type Transform) (Number%20of%20Enemies :type Integer))
  (for _index (range 0 (- Number%20of%20Enemies 1))
    (Game|SpawnActorfromClass Enemy SpawnTransform "Undefined" "MultiplyWithRoot" 0 0))
  (Variables|Default|SetTotal%20Spawned (+ (Variables|Default|GetTotal%20Spawned) (Variables|Default|GetNumber%20Of%20Enemies)))
  (Utilities|FlowControl|Delay (Variables|Default|GetSpawn%20Delay))
  (if (< (Variables|Default|GetTotal%20Spawned) (Variables|Default|GetMax%20Spawn))
    (CallFunction|MultiSpawn (Variables|Default|GetEnemy) (Transformation|GetActorTransform) (Variables|Default|GetNumber%20Of%20Enemies))))

(event Custom|SingleEnemy
  (params (Enemy :type Actor%20Class%20Reference) (SpawnTransform :type Transform))
  (Game|SpawnActorfromClass Enemy SpawnTransform "Undefined" "MultiplyWithRoot" 0 0))

(event Custom|ResetSpawning
  (Utilities|SingleSpawner))

(event EventBeginPlay
  (Utilities|SingleSpawner))

(fn ConstructionScript)