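; BP_StumbleCharacter is the armed player character in a zombie game, handling weapons, ammo, HUD, hit reactions and death.
; Tick polls grab, drop, sprint and aim states to swap socket-attached pickup weapons and toggle the crosshair.
; Semi or looping full-auto fire runs a spread trace, spawns barrel effects and casings, and adds recoil.
; Firing and sprinting report noise events, while death flags every zombie and mutant controller's blackboard.
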(event Custom|AttatchWeapon
  ;[1 1 1] Weapon Attach/Detach
  (if (not (Variables|Default|GetbIsWeaponAttached))
    (Class|BPIInteract|Interact(Message) (Utilities|Array|Get(acopy) (Collision|GetOverlappingActors "/Game/Stumble/NewGun/Props/Pickups/BP_PickupMaster.BP_PickupMaster_C" :!class /Script/Engine.Actor)) self)
    (UserInterface|Viewport|AddtoViewport (Variables|Default|GetAmmoWidget) 0)))

(event Custom|TakenDamage
  ;[1 1 1] Take Damage Animation
  (bind _asman_anim_bp (Utilities|Casting|CastToManAnimBP (Components|SkeletalMesh|GetAnimInstance (Variables|Character|GetMesh))))
  (Variables|/Game/Stumble/Assets/Character/Character/Animations/ManAnimBP.ManAnimBP_C|SetIsHit _asman_anim_bp true)
  (Utilities|FlowControl|Delay 3.0)
  (Variables|/Game/Stumble/Assets/Character/Character/Animations/ManAnimBP.ManAnimBP_C|SetIsHit _asman_anim_bp false))

(event Custom|DetachWeapon
  (bind _currentweapon (Variables|Default|GetCurrentWeapon))
  (bind _weaponmodel (Variables|/Game/Stumble/NewGun/Props/Weapons/BP_WeaponMaster.BP_WeaponMaster_C|GetWeaponModel _currentweapon))
  ;[1 1 1] Weapon Attach/Detach
  (Transformation|DetachFromActor _currentweapon "KeepWorld" "KeepWorld" "KeepWorld")
  (Collision|SetCollisionEnabled _weaponmodel "QueryAndPhysics")
  (Physics|SetSimulatePhysics _weaponmodel true)
  (Variables|Default|SetbIsWeaponAttached false)
  (switch Utilities|FlowControl|Switch|SwitchonEnum_WeaponName (Variables|/Game/Stumble/NewGun/Props/Weapons/BP_WeaponMaster.BP_WeaponMaster_C|GetWeapon%20Name _currentweapon)
    (:NewEnumerator1
      (Variables|Default|SetHasPistol false))
    (:NewEnumerator2
      (Variables|Default|SetHasRifle false)))
  (Widget|RemovefromParent (Variables|Default|GetAmmoWidget))
  (Utilities|FlowControl|Delay 1.0)
  (Actor|DestroyActor _currentweapon))

(event Custom|Spawn%20Weapon
  (params (Weapon%20To%20Spawn :type BP%20Weapon%20Master%20Class%20Reference))
  (bind _mesh (Variables|Character|GetMesh))
  ;[1 1 1] Attach Weapon/Swap weapon
  (Utilities|IsValid (Variables|Default|GetCurrentWeapon)
    (:Is%20Valid
      (Game|SpawnActorfromClass (Variables|/Game/Stumble/NewGun/Props/Weapons/BP_WeaponMaster.BP_WeaponMaster_C|GetPickup%20Class (Variables|Default|GetCurrentWeapon)) (Math|Transform|MakeTransform (+ (Transformation|GetActorLocation) (* (Transformation|GetActorForwardVector) "50.000000,50.000000,0.000000")) "0, 0, 0" "1.000000,1.000000,1.000000") "Undefined" "MultiplyWithRoot" 0 0 0)
      (Actor|DestroyActor (Variables|Default|GetCurrentWeapon)))
    (:Is%20Not%20Valid
      _))
  (bind _returnvalue (Game|SpawnActorfromClass Weapon%20To%20Spawn (Math|Transform|MakeTransform "0, 0, 0" "0, 0, 0" "1.000000,1.000000,1.000000") "Undefined" "MultiplyWithRoot" 0 0))
  (bind _output_get (Variables|Default|SetCurrentWeapon _returnvalue))
  (switch Utilities|FlowControl|Switch|SwitchonEnum_WeaponName (Variables|/Game/Stumble/NewGun/Props/Weapons/BP_WeaponMaster.BP_WeaponMaster_C|GetWeapon%20Name _output_get)
    (:NewEnumerator1
      (Transformation|AttachComponentToComponent _output_get _mesh "PistolSocket" "KeepRelative" "KeepRelative" "KeepRelative" true)
      (Variables|Default|SetHasPistol true)
      (Variables|Default|SetCurrentMag (Variables|/Game/Stumble/NewGun/Props/Weapons/BP_WeaponMaster.BP_WeaponMaster_C|GetMagazineSize (Variables|Default|GetCurrentWeapon)))
      (Variables|Default|SetPistolAmmo (Variables|/Game/Stumble/NewGun/Props/Weapons/BP_WeaponMaster.BP_WeaponMaster_C|GetMagazineSize (Variables|Default|GetCurrentWeapon)))
      (Variables|Default|SetAmmo (Variables|/Game/Stumble/NewGun/Props/Weapons/BP_WeaponMaster.BP_WeaponMaster_C|GetTotalAmmo (Variables|Default|GetCurrentWeapon))))
    (:NewEnumerator2
      (Transformation|AttachComponentToComponent _output_get _mesh "RifleSocket" "KeepRelative" "KeepRelative" "KeepRelative" true)
      (Variables|Default|SetHasRifle true)
      (Variables|Default|SetCurrentMag (Variables|/Game/Stumble/NewGun/Props/Weapons/BP_WeaponMaster.BP_WeaponMaster_C|GetMagazineSize (Variables|Default|GetCurrentWeapon)))
      (Variables|Default|SetAssaultRifleAmmo (Variables|/Game/Stumble/NewGun/Props/Weapons/BP_WeaponMaster.BP_WeaponMaster_C|GetMagazineSize (Variables|Default|GetCurrentWeapon)))
      (Variables|Default|SetAmmo (Variables|/Game/Stumble/NewGun/Props/Weapons/BP_WeaponMaster.BP_WeaponMaster_C|GetTotalAmmo (Variables|Default|GetCurrentWeapon)))))
  (Variables|Default|SetbIsWeaponAttached true))

(event Custom|Fire
  (params (CanFire :type Boolean))
  (bind _mesh (Variables|Character|GetMesh))
  (bind _currentweapon (Variables|Default|GetCurrentWeapon))
  (bind _returnvalue (Components|SkeletalMesh|GetAnimInstance _mesh))
  ;[1 1 1] Fire Weapon
  (Variables|Default|SetCanFire? CanFire)
  (bind _asstumble_characterbase (Utilities|Casting|CastToStumbleCharacterbase (Game|Player|GetPlayerPawn 0)))
  (Utilities|IsValid _currentweapon
    (:Is%20Valid
      (switch Utilities|FlowControl|Switch|SwitchonEnum_FireMode (Variables|/Game/Stumble/NewGun/Props/Weapons/BP_WeaponMaster.BP_WeaponMaster_C|GetFire%20Mode _currentweapon)
        (:NewEnumerator0
          (if (and (Variables|Default|GetCanFire?) (|Dead/Mag/Reloading/Aim _asstumble_characterbase))
            (CallFunction|LineTrace)
            (Class|BPIFire|Fire(Message) _currentweapon)
            (CallFunction|SetAmmo)
            (CallFunction|EjectCasing)
            (CallFunction|AddRecoil _returnvalue)
            (CallFunction|NoiseTriggered)))
        (:NewEnumerator1
          (if (and (Variables|Default|GetCanFire?) (|Dead/Mag/Reloading/Aim _asstumble_characterbase)) :!label _label
            (Class|BPIFire|Fire(Message) _currentweapon)
            (CallFunction|LineTrace)
            (CallFunction|SetAmmo)
            (CallFunction|EjectCasing)
            (CallFunction|AddRecoil _returnvalue)
            (CallFunction|NoiseTriggered)
            (Utilities|FlowControl|Delay 0.1)
            (goto _label)))))))

(event Custom|Line%20Trace
  (bind _currentweapon (Variables|Default|GetCurrentWeapon))
  (bind _spreadmultiplier (Variables|/Game/Stumble/NewGun/Props/Weapons/BP_WeaponMaster.BP_WeaponMaster_C|GetSpreadMultiplier _currentweapon))
  (bind _weaponmodel (Variables|/Game/Stumble/NewGun/Props/Weapons/BP_WeaponMaster.BP_WeaponMaster_C|GetWeaponModel _currentweapon))
  (bind _returnvalue (Transformation|GetSocketLocation _weaponmodel "barrel"))
  (bind _returnvalue_2 (Transformation|GetSocketRotation _weaponmodel "barrel"))
  (bind _returnvalue_3 (Math|Vector|GetForwardVector _returnvalue_2))
  ;[1 1 1] Bullet Projection
  (Collision|LineTraceByChannel _returnvalue (+ _returnvalue (* _returnvalue_3 1e+04) (Math|Vector|MakeVector (* (Math|Random|RandomFloatinRange -1.5e+02 1.5e+02) _spreadmultiplier) (* (Math|Random|RandomFloatinRange -1.5e+02 1.5e+02) _spreadmultiplier) (* (Math|Random|RandomFloatinRange -1.5e+02 1.5e+02) _spreadmultiplier))) "TraceTypeQuery1" true (Utilities|Array|MakeArray (Variables|Default|GetCurrentWeapon)) "None")
  (if true
    (Game|SpawnActorfromClass "/Game/Stumble/NewGun/BP_Bullet.BP_Bullet_C" (Math|Transform|MakeTransform _returnvalue (Math|Rotator|MakeRotfromX _returnvalue_3) "0.200000,0.200000,0.200000") "Undefined" "MultiplyWithRoot" 0 0)))

(event Custom|Reloading
  (bind _currentweapon (Variables|Default|GetCurrentWeapon))
  (bind _currentweapon_2 (Variables|Default|GetCurrentWeapon))
  (bind _weaponmodel (Variables|/Game/Stumble/NewGun/Props/Weapons/BP_WeaponMaster.BP_WeaponMaster_C|GetWeaponModel _currentweapon_2))
  ;[1 1 1] Reload Weapon
  (if (|Ammo/Reload/WeaponAttatched _currentweapon)
    (Variables|Default|SetReloading? true)
    (switch Utilities|FlowControl|Switch|SwitchonEnum_WeaponName (Variables|/Game/Stumble/NewGun/Props/Weapons/BP_WeaponMaster.BP_WeaponMaster_C|GetWeapon%20Name _currentweapon)
      (:NewEnumerator1
        (Animation|PlayAnimMontage "/Game/Stumble/Assets/Character/Character/Animations/Reload_Pistol_Montage.Reload_Pistol_Montage" 1.0 "None")
        (Components|Animation|PlayAnimation _weaponmodel "/Game/MilitaryWeapDark/Weapons/Anims/Reload_Pistol_W.Reload_Pistol_W" false))
      (:NewEnumerator2
        (Animation|PlayAnimMontage "/Game/Stumble/Assets/Character/Character/Animations/Reload_Rifle_Ironsights_Montage.Reload_Rifle_Ironsights_Montage" 1.0 "None")
        (Components|Animation|PlayAnimation _weaponmodel "/Game/MilitaryWeapDark/Weapons/Anims/Reload_Rifle_Ironsights_W.Reload_Rifle_Ironsights_W" false)))))

(event Custom|Eject%20Casing
  (bind _currentweapon (Variables|Default|GetCurrentWeapon))
  (bind _weaponmodel (Variables|/Game/Stumble/NewGun/Props/Weapons/BP_WeaponMaster.BP_WeaponMaster_C|GetWeaponModel _currentweapon))
  (bind _returnvalue (Transformation|GetSocketRotation _weaponmodel "AmmoEject"))
  (bind (_roll _pitch _yaw) (Math|Rotator|BreakRotator _returnvalue))
  ;[1 1 1] Ejects bullet casing
  (bind _returnvalue_2 (Game|SpawnActorfromClass (Variables|/Game/Stumble/NewGun/Props/Weapons/BP_WeaponMaster.BP_WeaponMaster_C|GetAmmoCasing _currentweapon) (Math|Transform|MakeTransform (Transformation|GetSocketLocation _weaponmodel "AmmoEject") (Math|Rotator|MakeRotator _roll (+ _pitch -9e+01) _yaw) "1.000000,1.000000,1.000000") "Undefined" "MultiplyWithRoot" 0 0))
  (Physics|AddImpulse (Variables|/Game/Stumble/NewGun/AmmoCasings/BP_AmmoCasingMaster.BP_AmmoCasingMaster_C|GetBulletCasing _returnvalue_2) (+ (* (Math|Vector|GetRightVector _returnvalue) (Math|Random|RandomFloatinRange 9e+01 1.5e+02)) (* (Transformation|GetVelocity) 0.8)) "None" true))

(event Custom|Set%20Ammo
  ;[1 1 1] UpdateAmmo
  (switch Utilities|FlowControl|Switch|SwitchonEnum_WeaponName (Variables|/Game/Stumble/NewGun/Props/Weapons/BP_WeaponMaster.BP_WeaponMaster_C|GetWeapon%20Name (Variables|Default|GetCurrentWeapon))
    (:NewEnumerator1
      (bind _result (Math|Integer|DecrementInt (Variables|Default|GetCurrentMag))
        (:%20%20
          (Variables|Default|SetPistolAmmo _result))))
    (:NewEnumerator2
      (bind _result_2 (Math|Integer|DecrementInt (Variables|Default|GetCurrentMag))
        (:%20%20
          (Variables|Default|SetAssaultRifleAmmo _result_2))))))

(event EventTick
  (params (DeltaSeconds :type Float%20%28single-precision%29))
  (bind _crosshair_widget (Variables|Default|GetCrosshair%20Widget))
  ;[1 1 1] Tick
  (Utilities|FlowControl|Sequence
    (:then_0
      (if (Class|StumbleCharacterbase|IsGrabbing)
        (CallFunction|AttatchWeapon)))
    (:then_1
      (if (Class|StumbleCharacterbase|IsDroppingWeapon)
        (CallFunction|DetachWeapon)))
    (:then_2
      (if (Class|StumbleCharacterbase|IsSprinting)
        (CallFunction|NoiseTriggered)))
    (:then_3
      (if (Class|StumbleCharacterbase|IsAiming)
        (UserInterface|Viewport|AddtoViewport _crosshair_widget 0)
        (else
          (Widget|RemovefromParent _crosshair_widget))))))

(event EventBeginPlay
  ;[1 1 1] Begin Play
  (bind _returnvalue (UserInterface|CreateWidget "/Game/Stumble/NewGun/AmmoWidget.AmmoWidget_C"))
  (Variables|Default|SetAmmoWidget _returnvalue)
  (bind _returnvalue_2 (UserInterface|CreateWidget "/Game/Stumble/NewGun/WBP_Crosshair.WBP_Crosshair_C"))
  (Variables|Default|SetCrosshair%20Widget _returnvalue_2)
  (bind _returnvalue_3 (UserInterface|CreateWidget "/Game/Stumble/Blueprints/Characters/WBP_HUD.WBP_HUD_C"))
  (UserInterface|Viewport|AddtoViewport _returnvalue_3 0))

(fn ConstructionScript)

(fn GetIsonLadder
  (return (Variables|Default|GetOnLadder)))

(fn SetDeathState
  (bind _returnvalue (UserInterface|CreateWidget "/Game/Stumble/Blueprints/Characters/WBP_DeathScreen.WBP_DeathScreen_C" (Game|GetPlayerController 0)))
  (UserInterface|Viewport|AddtoViewport _returnvalue 0)
  (Pawn|Components|CharacterMovement|DisableMovement (Variables|Character|GetCharacterMovement))
  (Variables|Default|SetIsDead true)
  (Utilities|FlowControl|Sequence
    (:then_0
      (bind _outactors (Actor|GetAllActorsOfClass "/Game/Stumble/Enemy/Controllers/SightChase/BP_ZombieController.BP_ZombieController_C"))
      (for _array_element _outactors
        (AI|Components|Blackboard|SetValueasBool (AI|GetBlackboard _array_element) (Utilities|Name|MakeLiteralName "IsPlayerDead") true)))
    (:then_1
      (bind _outactors_2 (Actor|GetAllActorsOfClass "/Game/Stumble/Enemy/Controllers/AutoChase/BP_ZombieControllerAutoChase.BP_ZombieControllerAutoChase_C"))
      (for _array_element_2 _outactors_2
        (AI|Components|Blackboard|SetValueasBool (AI|GetBlackboard _array_element_2) (Utilities|Name|MakeLiteralName "IsPlayerDead") true)))
    (:then_2
      (bind _outactors_3 (Actor|GetAllActorsOfClass "/Game/Stumble/Enemy/Controllers/SoundChase/BP_ZombieControllerSoundChase.BP_ZombieControllerSoundChase_C"))
      (for _array_element_3 _outactors_3
        (AI|Components|Blackboard|SetValueasBool (AI|GetBlackboard _array_element_3) (Utilities|Name|MakeLiteralName "IsPlayerDead") true)))
    (:then_3
      (bind _outactors_4 (Actor|GetAllActorsOfClass "/Game/Stumble/Enemy/Controllers/MutantBoss/BP_MutantController.BP_MutantController_C"))
      (for _array_element_4 _outactors_4
        (AI|Components|Blackboard|SetValueasBool (AI|GetBlackboard _array_element_4) (Utilities|Name|MakeLiteralName "IsPlayerDead") true)))))

(fn EnterRagdollState
  (Physics|SetSimulatePhysics (Variables|Character|GetMesh) true))

(fn Reload
  (bind _currentweapon (Variables|Default|GetCurrentWeapon))
  (switch Utilities|FlowControl|Switch|SwitchonEnum_WeaponName (Variables|/Game/Stumble/NewGun/Props/Weapons/BP_WeaponMaster.BP_WeaponMaster_C|GetWeapon%20Name _currentweapon)
    (:NewEnumerator1
      (bind _output_get (LocalVariables|SetTempAmmo (+ (Variables|Default|GetPistolAmmo) (Variables|Default|GetAmmo))))
      (Variables|Default|SetAmmo (- (Variables|Default|GetAmmo) (- (Math|Integer|Clamp(Integer) _output_get 0 (Variables|/Game/Stumble/NewGun/Props/Weapons/BP_WeaponMaster.BP_WeaponMaster_C|GetMagazineSize _currentweapon)) (Variables|Default|GetPistolAmmo)))))
    (:NewEnumerator2
      (bind _output_get_2 (LocalVariables|SetTempAmmo (+ (Variables|Default|GetAmmo) (Variables|Default|GetAssaultRifleAmmo))))
      (Variables|Default|SetAmmo (- (Variables|Default|GetAmmo) (- (Math|Integer|Clamp(Integer) _output_get_2 0 (Variables|/Game/Stumble/NewGun/Props/Weapons/BP_WeaponMaster.BP_WeaponMaster_C|GetMagazineSize _currentweapon)) (Variables|Default|GetAssaultRifleAmmo)))))))

(fn AddRecoil
  (params (self2 :type Object%20Object%20Reference))
  (bind _currentweapon (Variables|Default|GetCurrentWeapon))
  (Class|BPIAnimBPInt|IFRecoil(Message) self2 (Variables|/Game/Stumble/NewGun/Props/Weapons/BP_WeaponMaster.BP_WeaponMaster_C|GetRecoil%20Multi _currentweapon) (Variables|/Game/Stumble/NewGun/Props/Weapons/BP_WeaponMaster.BP_WeaponMaster_C|GetSide%20Recoil%20Multi _currentweapon) (Variables|/Game/Stumble/NewGun/Props/Weapons/BP_WeaponMaster.BP_WeaponMaster_C|GetKickback%20Multi _currentweapon) (Variables|/Game/Stumble/NewGun/Props/Weapons/BP_WeaponMaster.BP_WeaponMaster_C|GetKickside%20Multi _currentweapon) (Variables|/Game/Stumble/NewGun/Props/Weapons/BP_WeaponMaster.BP_WeaponMaster_C|GetKickup%20Multi _currentweapon)))

(fn NoiseTriggered
  (Class|AISenseHearing|ReportNoiseEvent (Transformation|GetActorLocation) 1.0 self 3e+03 "Sound"))