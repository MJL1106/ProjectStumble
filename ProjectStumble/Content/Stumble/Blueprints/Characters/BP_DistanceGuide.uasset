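; BP_DistanceGuide is a waypoint marker in Stumble that shows the player's distance to it in meters.
; Each Tick it measures from its widget component to the player character's mesh, hiding the widget beyond VisibleDistance and otherwise writing the truncated distance into WBP_DistanceToLocation.
; BeginPlay applies the configurable FontSize to that widget, and the actor destroys itself when a BP_StumbleCharacter overlaps its box.
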(event OnComponentBeginOverlap(Box)
  (params (OverlappedComponent :type Primitive%20Component%20Object%20Reference) (OtherActor :type Actor%20Object%20Reference) (OtherComp :type Primitive%20Component%20Object%20Reference) (OtherBodyIndex :type Integer) (bFromSweep :type Boolean) (SweepResult :type Hit%20Result%20Structure%20%28by%20ref%29))
  (Utilities|Casting|CastToBP_StumbleCharacter OtherActor)
  (Actor|DestroyActor))

(event EventBeginPlay
  (bind _aswbp_distance_to_location (Utilities|Casting|CastToWBP_DistanceToLocation (UserInterface|GetWidget (Variables|Default|GetWidget))))
  (Default|SetFontSize _aswbp_distance_to_location (Variables|Default|GetFontSize)))

(event EventTick
  (params (DeltaSeconds :type Float%20%28single-precision%29))
  (bind _widget (Variables|Default|GetWidget))
  (bind _asbp_stumble_character (Utilities|Casting|CastToBP_StumbleCharacter (Game|Player|GetPlayerPawn 0)))
  (if (<= (/ (Math|Vector|Distance(Vector) (Transformation|GetWorldLocation (Variables|Default|GetWidget)) (Transformation|GetWorldLocation (Variables|/Script/Engine.Character|GetMesh _asbp_stumble_character))) 1e+02) (Variables|Default|GetVisibleDistance))
    (Development|SetHiddeninGame _widget false false)
    (bind _aswbp_distance_to_location (Utilities|Casting|CastToWBP_DistanceToLocation (UserInterface|GetWidget _widget)))
    (Variables|/Script/UMG.TextBlock|SetText (Variables|/Game/Stumble/Blueprints/Characters/HUD/WBP_DistanceToLocation.WBP_DistanceToLocation_C|GetLocation _aswbp_distance_to_location) (Utilities|Text|ToText(String) (Utilities|String|Append (Utilities|String|ToString(Integer) (Math|Float|Truncate (/ (Math|Vector|Distance(Vector) (Transformation|GetWorldLocation (Variables|Default|GetWidget)) (Transformation|GetWorldLocation (Variables|/Script/Engine.Character|GetMesh _asbp_stumble_character))) 1e+02))) "m")))
    (else
      (Development|SetHiddeninGame (Variables|Default|GetWidget) true false))))

(fn ConstructionScript)