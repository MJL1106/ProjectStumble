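; BP_LevelTeleport is a trigger actor that moves the Stumble character between streamed levels behind a loading screen.
; Overlapping Teleporter disables input, shows WBP_LoadingScreen and asynchronously streams in LevelToLoad.
; It then snaps the character and control rotation to the PlayerSpawn component's transform.
; After a fixed delay, it removes the screen, restores input and unloads LevelToUnload.
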(event OnComponentBeginOverlap(Teleporter)
  (params (OverlappedComponent :type Primitive%20Component%20Object%20Reference) (OtherActor :type Actor%20Object%20Reference) (OtherComp :type Primitive%20Component%20Object%20Reference) (OtherBodyIndex :type Integer) (bFromSweep :type Boolean) (SweepResult :type Hit%20Result%20Structure%20%28by%20ref%29))
  (bind _returnvalue (Game|GetPlayerController 0))
  (bind _playerspawn (Variables|Default|GetPlayerSpawn))
  (bind _returnvalue_2 (Transformation|GetWorldRotation _playerspawn))
  (bind _asbp_stumble_character (Utilities|Casting|CastToBP_StumbleCharacter OtherActor))
  (bind _returnvalue_3 (UserInterface|CreateWidget "/Game/Stumble/Maps/WBP_LoadingScreen.WBP_LoadingScreen_C"))
  (Input|DisableInput _asbp_stumble_character _returnvalue)
  (UserInterface|Viewport|AddtoViewport _returnvalue_3 0)
  (Game|LoadStreamLevel(byName) (Variables|Default|GetLevelToLoad) true)
  (Transformation|SetActorLocationAndRotation _asbp_stumble_character (Transformation|GetWorldLocation _playerspawn) _returnvalue_2)
  (Pawn|SetControlRotation _returnvalue _returnvalue_2)
  (Utilities|FlowControl|Delay 2.0)
  (Widget|RemovefromParent _returnvalue_3)
  (Input|EnableInput _asbp_stumble_character (Game|GetPlayerController 0))
  (Game|UnloadStreamLevel(byName) (Variables|Default|GetLevelToUnload) false))

(fn ConstructionScript)