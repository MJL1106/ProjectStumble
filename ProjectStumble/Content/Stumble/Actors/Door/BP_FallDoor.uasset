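; BP_FallDoor is a door actor that swings open when its OpenDoor event is called.
; OpenDoor passes through a zero-length delay, then plays a timeline whose DoorOpen track rotates the Door component's relative roll from upright to a quarter turn.
; The Blueprint has no closing logic, and its BeginPlay, overlap and Tick events are disabled.
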(event EventBeginPlay
  (|CallParentFunction) ; This node is disabled and will not be called.\nDrag off pins to build functionality.
)

(event Collision|EventActorBeginOverlap
  (params (OtherActor :type Actor%20Object%20Reference))
  (|CallParentFunction OtherActor) ; This node is disabled and will not be called.\nDrag off pins to build functionality.
)

(event EventTick
  (params (DeltaSeconds :type Float%20%28single-precision%29))
  (|CallParentFunction DeltaSeconds) ; This node is disabled and will not be called.\nDrag off pins to build functionality.
)

(event EventOpenDoor
  (Utilities|FlowControl|Delay 0.0)
  (bind _dooropen (Timeline|Timeline Play)
    (:Update
      (Transformation|SetRelativeRotation (Variables|Default|GetDoor) (Math|Rotator|MakeRotator (Math|Float|Lerp 0.0 9e+01 _dooropen) 0.0 0.0) false false))))

(fn ConstructionScript
  (|CallParentFunction))