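; BP_MedKit is a health pickup for the Stumble character.
; When the character overlaps its Box, it adds HealAmount to PlayerHealth clamped between zero and one, plays a sound at the mesh and destroys itself.
; A separate WidgetVision overlap volume shows the kit's Widget while the character is inside and hides it on exit.
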(event OnComponentBeginOverlap(Box)
  (params (OverlappedComponent :type Primitive%20Component%20Object%20Reference) (OtherActor :type Actor%20Object%20Reference) (OtherComp :type Primitive%20Component%20Object%20Reference) (OtherBodyIndex :type Integer) (bFromSweep :type Boolean) (SweepResult :type Hit%20Result%20Structure%20%28by%20ref%29))
  (bind _asbp_stumble_character (Utilities|Casting|CastToBP_StumbleCharacter OtherActor))
  (Variables|/Game/Stumble/Blueprints/Characters/BP_StumbleCharacter.BP_StumbleCharacter_C|SetPlayerHealth _asbp_stumble_character (Math|Float|Clamp(Float) (+ (Variables|/Game/Stumble/Blueprints/Characters/BP_StumbleCharacter.BP_StumbleCharacter_C|GetPlayerHealth _asbp_stumble_character) (Variables|Default|GetHealAmount))))
  (Audio|PlaySoundatLocation "/Game/Stumble/Actors/Medkit/StartSimulate.StartSimulate" (Transformation|GetWorldLocation (Variables|Default|GetStaticMesh)) "0, 0, 0" 1.0 1.0 0.0 0 0 0 0)
  (Actor|DestroyActor))

(event OnComponentBeginOverlap(WidgetVision)
  (params (OverlappedComponent :type Primitive%20Component%20Object%20Reference) (OtherActor :type Actor%20Object%20Reference) (OtherComp :type Primitive%20Component%20Object%20Reference) (OtherBodyIndex :type Integer) (bFromSweep :type Boolean) (SweepResult :type Hit%20Result%20Structure%20%28by%20ref%29))
  (Utilities|Casting|CastToBP_StumbleCharacter OtherActor)
  (Rendering|SetVisibility (Variables|Default|GetWidget) true false))

(event OnComponentEndOverlap(WidgetVision)
  (params (OverlappedComponent :type Primitive%20Component%20Object%20Reference) (OtherActor :type Actor%20Object%20Reference) (OtherComp :type Primitive%20Component%20Object%20Reference) (OtherBodyIndex :type Integer))
  (Utilities|Casting|CastToBP_StumbleCharacter OtherActor)
  (Rendering|SetVisibility (Variables|Default|GetWidget) false false))

(fn ConstructionScript)