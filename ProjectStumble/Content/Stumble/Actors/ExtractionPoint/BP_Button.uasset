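; BP_Button is the extraction button actor that starts the escape countdown and ends the game when the player reaches the extraction point.
; A sphere overlap with BP_StumbleCharacter shows a prompt and enables interaction, and Tick polls the F key for the press.
; Pressing shows WBP_Timer with sound, then after a two-minute delay marks extraction ready and fades in helicopter audio.
; Overlapping ExtractionPoint once ready pauses the game and shows WBP_EndScreen.
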(event OnComponentBeginOverlap(Sphere)
  (params (OverlappedComponent :type Primitive%20Component%20Object%20Reference) (OtherActor :type Actor%20Object%20Reference) (OtherComp :type Primitive%20Component%20Object%20Reference) (OtherBodyIndex :type Integer) (bFromSweep :type Boolean) (SweepResult :type Hit%20Result%20Structure%20%28by%20ref%29))
  (Utilities|Casting|CastToBP_StumbleCharacter OtherActor)
  (if (not (Variables|Default|GetPressed?))
    (Rendering|SetVisibility (Variables|Default|GetPromptWidget) true false)
    (Variables|Default|SetCanInteract true)))

(event OnComponentBeginOverlap(ExtractionPoint)
  (params (OverlappedComponent :type Primitive%20Component%20Object%20Reference) (OtherActor :type Actor%20Object%20Reference) (OtherComp :type Primitive%20Component%20Object%20Reference) (OtherBodyIndex :type Integer) (bFromSweep :type Boolean) (SweepResult :type Hit%20Result%20Structure%20%28by%20ref%29))
  (bind _returnvalue (Game|GetPlayerController 0))
  (Utilities|Casting|CastToBP_StumbleCharacter OtherActor)
  (if (and (Variables|Default|GetPressed?) (Variables|Default|GetExtractionReady?))
    (Game|SetGamePaused true)
    (Widget|RemovefromParent (Variables|Default|GetTimerWidget))
    (bind _returnvalue_2 (UserInterface|CreateWidget "/Game/Stumble/Blueprints/Characters/HUD/WBP_EndScreen.WBP_EndScreen_C" _returnvalue))
    (UserInterface|Viewport|AddtoViewport _returnvalue_2 0)
    (Input|SetInputModeGameandUI _returnvalue 0 "DoNotLock" true false)
    (Variables|/Script/Engine.PlayerController|SetbShowMouseCursor _returnvalue true)))

(event OnComponentEndOverlap(Sphere)
  (params (OverlappedComponent :type Primitive%20Component%20Object%20Reference) (OtherActor :type Actor%20Object%20Reference) (OtherComp :type Primitive%20Component%20Object%20Reference) (OtherBodyIndex :type Integer))
  (Utilities|Casting|CastToBP_StumbleCharacter OtherActor)
  (Variables|Default|SetCanInteract false))

(event Custom|ButtonPressed
  (Rendering|SetVisibility (Variables|Default|GetPromptWidget) false false)
  (Variables|Default|SetPressed? true)
  (bind _returnvalue (UserInterface|CreateWidget "/Game/Stumble/Actors/ExtractionPoint/WBP_Timer.WBP_Timer_C" (Game|GetPlayerController 0)))
  (bind _output_get (Variables|Default|SetTimerWidget _returnvalue))
  (UserInterface|Viewport|AddtoViewport _output_get 0)
  (Components|Activation|Activate (Variables|Default|GetTimerSound) false)
  (Utilities|FlowControl|Delay 1.2e+02)
  (Variables|Default|SetExtractionReady? true)
  (Audio|Components|Audio|FadeIn (Variables|Default|GetHelicopterSound) 1e+01 1.0 0.0 "Linear" :!class /Script/Engine.AudioComponent))

(event EventTick
  (params (DeltaSeconds :type Float%20%28single-precision%29))
  (if (and (Variables|Default|GetCanInteract) (not (Variables|Default|GetPressed?)))
    (if (Game|Player|WasInputKeyJustPressed (Game|GetPlayerController 0) "F")
      (CallFunction|ButtonPressed))))

(fn ConstructionScript)