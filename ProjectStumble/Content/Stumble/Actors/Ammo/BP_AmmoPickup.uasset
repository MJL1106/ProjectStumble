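; BP_AmmoPickup is an ammo pickup actor that refills the Stumble character's ammo with a pistol or rifle amount, chosen by its AmmoType.
; Overlapping the Box adds ammo and destroys the pickup only if the character's current weapon matches that type, checked through WeaponName.
; A separate WidgetVision overlap volume shows the Widget while the character is inside and hides it on exit.
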(event OnComponentBeginOverlap(Box)
  (params (OverlappedComponent :type Primitive%20Component%20Object%20Reference) (OtherActor :type Actor%20Object%20Reference) (OtherComp :type Primitive%20Component%20Object%20Reference) (OtherBodyIndex :type Integer) (bFromSweep :type Boolean) (SweepResult :type Hit%20Result%20Structure%20%28by%20ref%29))
  (bind _asbp_stumble_character (Utilities|Casting|CastToBP_StumbleCharacter OtherActor))
  (switch Utilities|FlowControl|Switch|SwitchonE_AmmoType (Variables|Default|GetAmmoType)
    (:NewEnumerator0
      (Utilities|IsValid (Variables|/Game/Stumble/Blueprints/Characters/BP_StumbleCharacter.BP_StumbleCharacter_C|GetCurrentWeapon _asbp_stumble_character)
        (:Is%20Valid
          (switch Utilities|FlowControl|Switch|SwitchonEnum_WeaponName (Variables|/Game/Stumble/Weapons/Props/Weapons/BP_WeaponMaster.BP_WeaponMaster_C|GetWeapon%20Name (Variables|/Game/Stumble/Blueprints/Characters/BP_StumbleCharacter.BP_StumbleCharacter_C|GetCurrentWeapon _asbp_stumble_character))
            (:NewEnumerator1
              (Variables|/Game/Stumble/Blueprints/Characters/BP_StumbleCharacter.BP_StumbleCharacter_C|SetAmmo _asbp_stumble_character (+ (Variables|/Game/Stumble/Blueprints/Characters/BP_StumbleCharacter.BP_StumbleCharacter_C|GetAmmo _asbp_stumble_character) (Variables|Default|GetPistolAmmoAmount))))))))
    (:NewEnumerator1
      (Utilities|IsValid (Variables|/Game/Stumble/Blueprints/Characters/BP_StumbleCharacter.BP_StumbleCharacter_C|GetCurrentWeapon _asbp_stumble_character)
        (:Is%20Valid
          (switch Utilities|FlowControl|Switch|SwitchonEnum_WeaponName (Variables|/Game/Stumble/Weapons/Props/Weapons/BP_WeaponMaster.BP_WeaponMaster_C|GetWeapon%20Name (Variables|/Game/Stumble/Blueprints/Characters/BP_StumbleCharacter.BP_StumbleCharacter_C|GetCurrentWeapon _asbp_stumble_character))
            (:NewEnumerator2
              (Variables|/Game/Stumble/Blueprints/Characters/BP_StumbleCharacter.BP_StumbleCharacter_C|SetAmmo _asbp_stumble_character (+ (Variables|/Game/Stumble/Blueprints/Characters/BP_StumbleCharacter.BP_StumbleCharacter_C|GetAmmo _asbp_stumble_character) (Variables|Default|GetRifleAmmoAmount)))))))))
  (Actor|DestroyActor))

(event OnComponentBeginOverlap(WidgetVision)
  (params (OverlappedComponent :type Primitive%20Component%20Object%20Reference) (OtherActor :type Actor%20Object%20Reference) (OtherComp :type Primitive%20Component%20Object%20Reference) (OtherBodyIndex :type Integer) (bFromSweep :type Boolean) (SweepResult :type Hit%20Result%20Structure%20%28by%20ref%29))
  (Utilities|Casting|CastToBP_StumbleCharacter OtherActor)
  (Rendering|SetVisibility (Variables|Default|GetWidget) true false))

(event OnComponentEndOverlap(WidgetVision)
  (params (OverlappedComponent :type Primitive%20Component%20Object%20Reference) (OtherActor :type Actor%20Object%20Reference) (OtherComp :type Primitive%20Component%20Object%20Reference) (OtherBodyIndex :type Integer))
  (Utilities|Casting|CastToBP_StumbleCharacter OtherActor)
  (Rendering|SetVisibility (Variables|Default|GetWidget) false false))

(fn ConstructionScript)