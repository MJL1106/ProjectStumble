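; BP_DoorKnockdownSound is a one-shot trigger that plays a sound and signals the level's fall doors.
; The first overlap of its Box, by any actor that can trigger it, activates the Audio component and sets AlreadyPlayed to block repeats.
; It then finds every BP_FallDoor with GetAllActorsOfClass and calls OpenDoorMessage on each, so one trigger affects all of them.
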(event OnComponentBeginOverlap(Box)
  (params (OverlappedComponent :type Primitive%20Component%20Object%20Reference) (OtherActor :type Actor%20Object%20Reference) (OtherComp :type Primitive%20Component%20Object%20Reference) (OtherBodyIndex :type Integer) (bFromSweep :type Boolean) (SweepResult :type Hit%20Result%20Structure%20%28by%20ref%29))
  (if (not (Variables|Default|GetAlreadyPlayed))
    (Components|Activation|Activate (Variables|Default|GetAudio) false)
    (Variables|Default|SetAlreadyPlayed true)
    (bind _outactors (Actor|GetAllActorsOfClass "/Game/Stumble/Actors/Door/BP_FallDoor.BP_FallDoor_C"))
    (for _array_element _outactors
      (Class|BPIOpenDoor|OpenDoor(Message) _array_element))))

(event EventBeginPlay
  (|CallParentFunction) ; This node is disabled and will not be called.\nDrag off pins to build functionality.
)

(event Collision|EventActorBeginOverlap
  (params (OtherActor :type Actor%20Object%20Reference))
  (|CallParentFunction OtherActor) ; This node is disabled and will not be called.\nDrag off pins to build functionality.
)

(event EventTick
  (params (DeltaSeconds :type Float%20%28single-precision%29))
  (|CallParentFunction DeltaSeconds) ; This node is disabled and will not be called.\nDrag off pins to build functionality.
)

(fn ConstructionScript
  (|CallParentFunction))