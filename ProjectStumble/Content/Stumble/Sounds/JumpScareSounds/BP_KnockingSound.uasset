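; BP_KnockingSound is a jump-scare sound trigger that plays a knocking sound when something enters its box volume.
; The first Box overlap activates the Audio component, immediately starts a long linear fade to silence, and sets AlreadyPlayed so it never replays.
; Any end overlap deactivates the audio, and neither overlap event checks which actor caused it.
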(event OnComponentBeginOverlap(Box)
  (params (OverlappedComponent :type Primitive%20Component%20Object%20Reference) (OtherActor :type Actor%20Object%20Reference) (OtherComp :type Primitive%20Component%20Object%20Reference) (OtherBodyIndex :type Integer) (bFromSweep :type Boolean) (SweepResult :type Hit%20Result%20Structure%20%28by%20ref%29))
  (if (not (Variables|Default|GetAlreadyPlayed))
    (Components|Activation|Activate (Variables|Default|GetAudio) false)
    (Audio|Components|Audio|FadeOut (Variables|Default|GetAudio) 1e+01 0.0 "Linear" :!class /Script/Engine.AudioComponent)
    (Variables|Default|SetAlreadyPlayed true)))

(event OnComponentEndOverlap(Box)
  (params (OverlappedComponent :type Primitive%20Component%20Object%20Reference) (OtherActor :type Actor%20Object%20Reference) (OtherComp :type Primitive%20Component%20Object%20Reference) (OtherBodyIndex :type Integer))
  (Components|Activation|Deactivate (Variables|Default|GetAudio)))

(event EventBeginPlay
  (|CallParentFunction) ; This node is disabled and will not be called.\nDrag off pins to build functionality.
)

(event Collision|EventActorBeginOverlap
  (params (OtherActor :type Actor%20Object%20Reference))
  (|CallParentFunction OtherActor) ; This node is disabled and will not be called.\nDrag off pins to build functionality.
)

(event EventTick
  (params (DeltaSeconds :type Float%20%28single-precision%29))
  (|CallParentFunction DeltaSeconds) ; This node is disabled and will not be called.\nDrag off pins to build functionality.
)

(fn ConstructionScript
  (|CallParentFunction))