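; BP_LevelAmbience is an actor that starts the background ambience sound for one of three levels in Stumble.
; On BeginPlay it switches on LevelChoice and activates the matching Level1, Level2 or Level3 component.
; A parallel switch that would fade out the selected component is not connected to any event, so EndPlay does nothing.
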(event EventBeginPlay
  (switch Utilities|FlowControl|Switch|SwitchonE_SoundChoice (Variables|Default|GetLevelChoice)
    (:NewEnumerator0
      (Components|Activation|Activate (Variables|Default|GetLevel1) false))
    (:NewEnumerator1
      (Components|Activation|Activate (Variables|Default|GetLevel2) false))
    (:NewEnumerator2
      (Components|Activation|Activate (Variables|Default|GetLevel3) false))))

(event EventEndPlay
  (params (EndPlayReason :type EEndPlayReason%20Enum :default "Destroyed")))

(fn ConstructionScript)