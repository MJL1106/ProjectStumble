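; EnemyBP is an enemy in the Stumble game that chases the player character and can be killed by damage.
; On BeginPlay it caches the player's BP_StumbleCharacter, starts the chase and picks a random walk speed, though the last speed option is never selected.
; ChasePlayer re-issues AI Move To whenever it succeeds or fails.
; AnyDamage lowers clamped Health and plays a sound, destroying the actor at zero.
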(event Custom|Chase%20Player
  (params (Player%20To%20Chase :type BP%20Stumble%20Character%20Object%20Reference))
  (AI|AIMoveTo self "0, 0, 0" Player%20To%20Chase 5.0 false
    (:OnSuccess
      _)
    (:OnFail
      _))
  (CallFunction|ChasePlayer (Variables|Default|GetChar%20Ref)))

(event EventBeginPlay
  (bind _asbp_stumble_character (Utilities|Casting|CastToBP_StumbleCharacter (Game|GetPlayerCharacter 0)))
  (bind _output_get (Variables|Default|SetChar%20Ref _asbp_stumble_character))
  (CallFunction|ChasePlayer _output_get)
  (Variables|/Script/Engine.CharacterMovementComponent|SetMaxWalkSpeed (Variables|Character|GetCharacterMovement) (Utilities|Select :Index (Math|Random|RandomInteger 3) :Option%200 2e+02 :Option%201 2.5e+02 :Option%202 3e+02 :Option%203 3.5e+02)))

(event Game|Damage|EventAnyDamage
  (params (Damage :type Float%20%28single-precision%29) (DamageType :type Damage%20Type%20Object%20Reference) (InstigatedBy :type Controller%20Object%20Reference) (DamageCauser :type Actor%20Object%20Reference))
  (bind _returnvalue (Transformation|GetActorLocation))
  (bind _output_get (Variables|Default|SetHealth (Math|Float|Clamp(Float) (- (Variables|Default|GetHealth) Damage) 0.0 1e+02)))
  (if (== _output_get 0.0)
    (Audio|PlaySoundatLocation 0 _returnvalue "0, 0, 0" 1.0 1.0 0.0 0 0 0 0)
    (Actor|DestroyActor)
    (else
      (Audio|PlaySoundatLocation 0 _returnvalue "0, 0, 0" 1.0 1.0 0.0 0 0 0 0))))

(fn ConstructionScript)