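; Mutant boss enemy that roars at the player on spawn, then runs its behavior tree.
; Short, medium and slam attacks roll random damage, which DamagePlayer applies within each attack's range.
; The slam leaps on a projectile arc toward the player's predicted position.
; It also manages a camera-facing health bar, damage popups, proximity ambient sounds, ragdoll death and blackboard death flags for itself and the player.
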(event Custom|ShortAttack
  ;[1 1 1] Short Attack
  (Animation|Montage|PlayMontage (Variables|Character|GetMesh) "/Game/Stumble/Enemy/MutantBoss/Animations/MutantAttack3.MutantAttack3"
    (:then
      (Variables|Default|SetAttackDamage (Math|Random|RandomIntegerinRange 20 25)))))

(event Custom|PlayerDead
  ;[1 1 1] Player Died
  (bind _asmutant_anim_bp (Utilities|Casting|CastToMutantAnimBP (Components|SkeletalMesh|GetAnimInstance (Variables|Character|GetMesh))))
  (Variables|/Game/Stumble/Enemy/MutantBoss/Animations/MutantAnimBP.MutantAnimBP_C|SetIsPlayerDead _asmutant_anim_bp true))

(event Custom|SlamAttack
  (bind _returnvalue (Transformation|GetActorLocation))
  ;[1 1 1] Slam Attack
  (Variables|Default|SetAttackDamage (Math|Random|RandomIntegerinRange 35 50))
  (Variables|Default|SetSlamAttack? true)
  (bind _location (CallFunction|CalculateFutureActorLocation (Game|GetPlayerCharacter 0) 1.0))
  (bind _outlaunchvelocity (Game|SuggestProjectileVelocityCustomArc _returnvalue (Math|Vector|MakeVector (.x _location) (.y _location) (+ (.z _location) 5e+01)) 0.0 0.5))
  (Transformation|SetActorRotation (Math|Interpolation|RInterpTo (Transformation|GetActorRotation) (Math|Rotator|FindLookatRotation _returnvalue (Math|Vector|MakeVector (.x _location) (.y _location) (+ (.z _location) 5e+01))) (Utilities|Time|GetWorldDeltaSeconds) 1e+01))
  (Animation|PlayAnimMontage "/Game/Stumble/Enemy/MutantBoss/Animations/MutantAttack2.MutantAttack2" 1.0 "None")
  (Utilities|FlowControl|Delay 0.4)
  (Character|LaunchCharacter _outlaunchvelocity false false)
  (EventDispatchers|BindEventtoLandedDelegate (delegate Custom|OnLand)))

(event Custom|OnLand
  (params (Hit :type Hit%20Result%20Structure%20%28by%20ref%29))
  ;[1 1 1] Slam Attack
  (EventDispatchers|UnbindEventfromLandedDelegate (delegate Custom|OnLand))
  (Components|Movement|StopMovementImmediately (Variables|Character|GetCharacterMovement))
  (Utilities|FlowControl|Delay 2.6)
  (Variables|Default|SetSlamAttack? false))

(event Custom|Damage%20Player
  ;[1 1 1] Damage Player
  (Utilities|DamagePlayer))

(event Custom|MediumRangeAttack
  ;[1 1 1] Mid Range Attack
  (Variables|Default|SetMediumAttack true)
  (Animation|PlayAnimMontage "/Game/Stumble/Enemy/MutantBoss/Animations/MutantAttack1.MutantAttack1" 1.0 "None")
  (Variables|Default|SetAttackDamage (Math|Random|RandomIntegerinRange 25 35))
  (Utilities|FlowControl|Delay 2.6)
  (Variables|Default|SetMediumAttack false))

(event EventTick
  (params (DeltaSeconds :type Float%20%28single-precision%29))
  (bind _healthbar (Variables|Default|GetHealthBar))
  (bind _aswbp_health_enemy (Utilities|Casting|CastToWBP_HealthEnemy (UserInterface|GetWidget (Variables|Default|GetHealthBar))))
  (Progress|SetPercent (Variables|/Game/Stumble/Enemy/Widgets/WBP_HealthEnemy.WBP_HealthEnemy_C|GetHealthBar _aswbp_health_enemy) (/ (Variables|Default|GetHealth) (Variables|Default|GetMaxHealth)))
  (Transformation|SetWorldRotation _healthbar (Math|Rotator|FindLookatRotation (Transformation|GetWorldLocation _healthbar) (Transformation|GetWorldLocation (Variables|/Script/Engine.PlayerCameraManager|GetTransformComponent (Game|GetPlayerCameraManager 0)))) false false))

(event Game|Damage|EventAnyDamage
  (params (Damage :type Float%20%28single-precision%29) (DamageType :type Damage%20Type%20Object%20Reference) (InstigatedBy :type Controller%20Object%20Reference) (DamageCauser :type Actor%20Object%20Reference))
  (bind _returnvalue (Transformation|GetActorLocation))
  ;[1 1 1] Deal Damage To Zombie
  (if (not (Variables|Default|GetIsDead?))
    (bind _output_get (Variables|Default|SetHealth (Math|Float|Clamp(Float) (- (Variables|Default|GetHealth) Damage) 0.0 (Variables|Default|GetMaxHealth))))
    (if (== _output_get 0.0)
      (Audio|PlaySoundatLocation "/Game/Stumble/Enemy/Sounds/Impact/SC_Hit.SC_Hit" _returnvalue "0, 0, 0" 1.0 1.0 0.0 0 0 0 0)
      (Components|Activation|Deactivate (Variables|Default|GetSC_AmbientNoises))
      (Audio|PlaySoundatLocation "/Game/Zombie/Sound/Entity/SC_Entity_Death.SC_Entity_Death" _returnvalue "0, 0, 0" 1.0 1.0 0.0 0 0 0 0)
      (Pawn|Components|CharacterMovement|DisableMovement (Variables|Character|GetCharacterMovement))
      (Variables|Default|SetIsDead? true)
      (Development|SetHiddeninGame (Variables|Default|GetHealthBar) true false)
      (Physics|SetSimulatePhysics (Variables|Character|GetMesh) true)
      (Collision|SetCollisionEnabled (Variables|Collision|GetCapsuleComponent) "NoCollision")
      (AI|Components|Blackboard|SetValueasBool (AI|GetBlackboard 0) (Utilities|Name|MakeLiteralName "IsZombieDead") true)
      (Utilities|FlowControl|Delay 15.0)
      (Actor|DestroyActor)
      (else
        (Audio|PlaySoundatLocation "/Game/Stumble/Enemy/Sounds/Impact/SC_Hit.SC_Hit" _returnvalue "0, 0, 0" 1.0 1.0 0.0 0 0 0 0)
        (Game|SpawnActorfromClass "/Game/Stumble/Enemy/Widgets/BP_DmgAmt.BP_DmgAmt_C" (Transformation|GetActorTransform) "Undefined" "MultiplyWithRoot" 0 Damage 0)))))

(event EventBeginPlay
  (|RoarToPlayer)
  (Utilities|PlayZombieSounds))

(fn ConstructionScript)

(fn CalculateFutureActorLocation
  (params (Actor :type Actor%20Object%20Reference) (Time :type Float%20%28double-precision%29))
  (return (+ (Transformation|GetActorLocation Actor) (* (* (Transformation|GetVelocity Actor) "1.000000,1.000000,0.000000") Time))))