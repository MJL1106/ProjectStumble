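; AI controller for a sound-chasing zombie, which runs the ZombieBTSoundChase behavior tree on BeginPlay.
; AI perception updates about the player's BP_StumbleCharacter are written to the blackboard for that tree.
; Stimuli tagged "Sound" set HasHeardSound and SoundLocation, while any other stimulus sets HasSpottedPlayer, with both flags following whether sensing succeeded.
; Debug strings print the stimulus tag and heard sounds.
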(event OnTargetPerceptionUpdated(AIPerception)
  (params (Actor :type Actor%20Object%20Reference) (Stimulus :type AI%20Stimulus%20Structure))
  (bind _returnvalue (AI|GetBlackboard 0))
  (for _array_element (Utilities|Array|MakeArray Stimulus)
    (Variables|Default|SetHasSensed (.bSuccessfullySensed (Utilities|Struct|BreakAIStimulus _array_element)))
    (Utilities|Casting|CastToBP_StumbleCharacter Actor)
    (Development|PrintString (Utilities|String|ToString(Name) (.Tag (Utilities|Struct|BreakAIStimulus _array_element))))
    (if (== (.Tag (Utilities|Struct|BreakAIStimulus _array_element)) "Sound")
      (Development|PrintString "HEARD SOUND")
      (AI|Components|Blackboard|SetValueasBool _returnvalue (Utilities|Name|MakeLiteralName "HasHeardSound") (Variables|Default|GetHasSensed))
      (AI|Components|Blackboard|SetValueasVector _returnvalue (Utilities|Name|MakeLiteralName "SoundLocation") (.StimulusLocation (Utilities|Struct|BreakAIStimulus _array_element)))
      (else
        (AI|Components|Blackboard|SetValueasBool (AI|GetBlackboard 0) (Utilities|Name|MakeLiteralName "HasSpottedPlayer") (Variables|Default|GetHasSensed))))))

(event EventBeginPlay
  (AI|RunBehaviorTree "/Game/Stumble/Enemy/AI/BehaviourTrees/SoundChase/ZombieBTSoundChase.ZombieBTSoundChase"))

(fn ConstructionScript)