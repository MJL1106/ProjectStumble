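; BP_ZombieController is the AI controller for sight-chase zombies in Stumble.
; It runs the ZombieBT behavior tree on BeginPlay.
; When AI perception updates on the player character, it writes the sensed result to the HasSpottedPlayer blackboard key.
; It then calls AlertedSound on the controlled zombie, whether the player was gained or lost.
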(event OnTargetPerceptionUpdated(AIPerception)
  (params (Actor :type Actor%20Object%20Reference) (Stimulus :type AI%20Stimulus%20Structure))
  (Variables|Default|SetHasSensed (.bSuccessfullySensed (Utilities|Struct|BreakAIStimulus Stimulus)))
  (Utilities|Casting|CastToBP_StumbleCharacter Actor)
  (AI|Components|Blackboard|SetValueasBool (AI|GetBlackboard 0) (Utilities|Name|MakeLiteralName "HasSpottedPlayer") (Variables|Default|GetHasSensed))
  (bind _aszombie_character_sight_chase (Utilities|Casting|CastToZombieCharacter_SightChase (Pawn|GetControlledPawn)))
  (Default|AlertedSound _aszombie_character_sight_chase))

(event EventBeginPlay
  (AI|RunBehaviorTree "/Game/Stumble/Enemy/AI/BehaviourTrees/SightChase/ZombieBT.ZombieBT"))

(fn ConstructionScript)