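; BP_PickupMaster is a pickup Blueprint, apparently a shared base, that toggles a widget as overlaps occur on its WidgetVision component.
; On overlap begin it casts player 0's pawn to StumbleCharacterbase and shows the widget only if no weapon is attached.
; On overlap end it hides the widget.
; Neither event checks which actor overlapped, and no pickup logic lives in these graphs.
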(event OnComponentBeginOverlap(WidgetVision)
  (params (OverlappedComponent :type Primitive%20Component%20Object%20Reference) (OtherActor :type Actor%20Object%20Reference) (OtherComp :type Primitive%20Component%20Object%20Reference) (OtherBodyIndex :type Integer) (bFromSweep :type Boolean) (SweepResult :type Hit%20Result%20Structure%20%28by%20ref%29))
  (bind _asstumble_characterbase (Utilities|Casting|CastToStumbleCharacterbase (Game|Player|GetPlayerPawn 0)))
  (if (Variables|/Script/ProjectStumble.StumbleCharacterbase|GetbIsWeaponAttached _asstumble_characterbase)
    (Rendering|SetVisibility (Variables|Default|GetWidget) false false)
    (else
      (Rendering|SetVisibility (Variables|Default|GetWidget) true false))))

(event OnComponentEndOverlap(WidgetVision)
  (params (OverlappedComponent :type Primitive%20Component%20Object%20Reference) (OtherActor :type Actor%20Object%20Reference) (OtherComp :type Primitive%20Component%20Object%20Reference) (OtherBodyIndex :type Integer))
  (Rendering|SetVisibility (Variables|Default|GetWidget) false false))

(event EventBeginPlay)

(event Collision|EventActorBeginOverlap
  (params (OtherActor :type Actor%20Object%20Reference)))

(event EventTick
  (params (DeltaSeconds :type Float%20%28single-precision%29)))

(fn ConstructionScript)