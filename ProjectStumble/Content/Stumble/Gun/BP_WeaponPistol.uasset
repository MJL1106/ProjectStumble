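; Pistol pickup actor for the Stumble character, with a widget that marks its location.
; Overlapping the pickup capsule passes the barrel sphere and weapon reference to BP_StumbleCharacter and enables pickup on it.
; A separate WidgetVision overlap shows the widget unless the player pawn already has a weapon attached, and hides it when the overlap ends.
; Firing is not handled here.
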(event OnComponentBeginOverlap(WidgetVision)
  (params (OverlappedComponent :type Primitive%20Component%20Object%20Reference) (OtherActor :type Actor%20Object%20Reference) (OtherComp :type Primitive%20Component%20Object%20Reference) (OtherBodyIndex :type Integer) (bFromSweep :type Boolean) (SweepResult :type Hit%20Result%20Structure%20%28by%20ref%29))
  ;[1 1 1] Displays Location Widget
  (bind _asstumble_characterbase (Utilities|Casting|CastToStumbleCharacterbase (Game|Player|GetPlayerPawn 0)))
  (if (Variables|/Script/ProjectStumble.StumbleCharacterbase|GetbIsWeaponAttached _asstumble_characterbase)
    (Rendering|SetVisibility (Variables|Default|GetWidget) false false)
    (else
      (Rendering|SetVisibility (Variables|Default|GetWidget) true false))))

(event OnComponentBeginOverlap(PickupCapsule)
  (params (OverlappedComponent :type Primitive%20Component%20Object%20Reference) (OtherActor :type Actor%20Object%20Reference) (OtherComp :type Primitive%20Component%20Object%20Reference) (OtherBodyIndex :type Integer) (bFromSweep :type Boolean) (SweepResult :type Hit%20Result%20Structure%20%28by%20ref%29))
  ;[1 1 1] Can Interact with weapon
  (bind _asbp_stumble_character (Utilities|Casting|CastToBP_StumbleCharacter OtherActor))
  (Default|SetSphereRef _asbp_stumble_character (Variables|Default|GetBarrelSphere))
  (Default|SetWeapon _asbp_stumble_character (Variables|Default|GetSelfReference))
  (Default|SetCanPickup _asbp_stumble_character true))

(event OnComponentEndOverlap(PickupCapsule)
  (params (OverlappedComponent :type Primitive%20Component%20Object%20Reference) (OtherActor :type Actor%20Object%20Reference) (OtherComp :type Primitive%20Component%20Object%20Reference) (OtherBodyIndex :type Integer))
  ;[1 1 1] Can Interact with weapon
  (Utilities|Casting|CastToBP_StumbleCharacter OtherActor)
  (Variables|Default|SetbCanPickup false))

(event OnComponentEndOverlap(WidgetVision)
  (params (OverlappedComponent :type Primitive%20Component%20Object%20Reference) (OtherActor :type Actor%20Object%20Reference) (OtherComp :type Primitive%20Component%20Object%20Reference) (OtherBodyIndex :type Integer))
  ;[1 1 1] Displays Location Widget
  (Rendering|SetVisibility (Variables|Default|GetWidget) false false))

(event EventBeginPlay
  (Variables|Default|SetSelfReference self)
  (Variables|Default|SetSphereRef (Variables|Default|GetBarrelSphere)))

(fn ConstructionScript)